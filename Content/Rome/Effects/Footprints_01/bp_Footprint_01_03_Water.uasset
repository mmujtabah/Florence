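; Water variant of a footprint effect actor that reveals a decal, optionally with a Niagara particle effect.
; On BeginPlay it hides the decal at zero scale and waits a configurable delay, then a timeline drives the decal's scale.
; With particles enabled, it spawns the Niagara system at the decal with raised translucent sort priority, and the timeline plays only if that system asset is valid.
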(event `self.ReceiveBeginPlay`
  (bind _niagaraparticle (`self.NiagaraParticle`))
  (`SceneComponent.SetWorldScale3D` (`self.Decal`) (0.0 0.0 0.0))
  (`KismetSystemLibrary.Delay` (`self.Delay`))
  (if (`self.UseParticle`)
    (`/Engine/EditorBlueprintResources/StandardMacros.IsValid` _niagaraparticle
      (:`Is Valid`
        (bind _returnvalue (`NiagaraFunctionLibrary.SpawnSystemAtLocation` _niagaraparticle (`SceneComponent.K2_GetComponentLocation` (`self.Decal`))))
        (`PrimitiveComponent.SetTranslucentSortPriority` _returnvalue 1)
        (bind (_direction _decalsize) (`Timeline|Timeline_0` :!label _label)
          (:`Update`
            (`SceneComponent.SetWorldScale3D` (`self.Decal`) (`KismetMathLibrary.Conv_DoubleToVector` _decalsize))))))
    (else
      (goto _label))))

(fn `UserConstructionScript`)