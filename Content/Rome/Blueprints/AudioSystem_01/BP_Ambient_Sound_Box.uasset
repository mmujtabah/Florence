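; Box-shaped ambient sound volume that plays four-channel (front/rear, left/right) audio through emitters that follow the player.
; Each tick offsets four points along world axes from the active FPP or TPP camera, then clamps them in box space to position the emitters.
; Tick runs fastest after the character enters and slows by distance after exit, though nested checks leave the two slowest tiers unreachable.
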(event `self.Box.OnComponentBeginOverlap`
  (params (OverlappedComponent :type "PrimitiveComponent Object Reference") (OtherActor :type "Actor Object Reference") (OtherComp :type "PrimitiveComponent Object Reference") (OtherBodyIndex :type Integer) (bFromSweep :type Boolean) (SweepResult :type "HitResult Structure (by ref)"))
  (cast `/Game/Rome/Demo/PawnUE5/Demo/EpicContent/ThirdPersonBP/Blueprints/BP_ThirdPersonCharacter` OtherActor)
  (set `self.AllowOptimization` false)
  (`self.SetActorTickInterval` 0.05))

(event `self.Box.OnComponentEndOverlap`
  (params (OverlappedComponent :type "PrimitiveComponent Object Reference") (OtherActor :type "Actor Object Reference") (OtherComp :type "PrimitiveComponent Object Reference") (OtherBodyIndex :type Integer))
  (cast `/Game/Rome/Demo/PawnUE5/Demo/EpicContent/ThirdPersonBP/Blueprints/BP_ThirdPersonCharacter` OtherActor)
  (set `self.AllowOptimization` true))

(event `self.ReceiveTick`
  (params (DeltaSeconds :type "Float (single-precision)"))
  (bind (_front _right _back _left) (`self.CalculateEmitterPositions` (`self.CurrentPawnLocation`) (struct) (`self.EmmiterPointsOffset`)))
  (bind _returnvalue (`SceneComponent.K2_GetComponentLocation` (`Character.Mesh` (`self.Character Reference`))))
  (bind _returnvalue_2 (`KismetMathLibrary.VSize` (- (`PrimitiveComponent.GetClosestPointOnCollision` (`self.Box`) _returnvalue "head") _returnvalue)))
  (`|ExecutionSequence`
    (:`then_0`
      (if (`ActorComponent.IsActive` (`/Game/Rome/Demo/PawnUE5/Demo/EpicContent/ThirdPersonBP/Blueprints/BP_ThirdPersonCharacter.FPPCamera` (`self.Character Reference`)))
        (set `self.CurrentPawnLocation` (`SceneComponent.K2_GetComponentLocation` (`/Game/Rome/Demo/PawnUE5/Demo/EpicContent/ThirdPersonBP/Blueprints/BP_ThirdPersonCharacter.FPPCamera` (`self.Character Reference`))))
        (else
          (set `self.CurrentPawnLocation` (`SceneComponent.K2_GetComponentLocation` (`/Game/Rome/Demo/PawnUE5/Demo/EpicContent/ThirdPersonBP/Blueprints/BP_ThirdPersonCharacter.TPPCamera` (`self.Character Reference`))))))
      (`|ExecutionSequence`
        (:`then_0`
          ;[1 1 1] Clamped Emitter Points
          (`self.ConstrainPoint` _front (struct :`R` 1.0 :`A` 1.0) (`self.FL`))
          (if (`self.DrawDebug`)
            ;[1 1 1] Debug Only
            (`KismetSystemLibrary.DrawDebugPoint` (0.0 0.0 0.0) 30.0 (struct :`R` 1.0 :`G` 0.041194 :`A` 1.0))))
        (:`then_1`
          (`self.ConstrainPoint` _right (struct :`R` 1.0 :`G` 0.889721 :`A` 1.0) (`self.FR`))
          (if (`self.DrawDebug`)
            (`KismetSystemLibrary.DrawDebugPoint` (0.0 0.0 0.0) 30.0 (struct :`R` 1.0 :`G` 0.867982 :`A` 1.0))))
        (:`then_2`
          (`self.ConstrainPoint` _back (struct :`R` 0.083052 :`G` 1.0 :`A` 1.0) (`self.RR`))
          (if (`self.DrawDebug`)
            (`KismetSystemLibrary.DrawDebugPoint` (0.0 0.0 0.0) 30.0 (struct :`R` 0.115801 :`G` 1.0 :`B` 0.104591 :`A` 1.0))))
        (:`then_3`
          (`self.ConstrainPoint` _left (struct :`G` 0.914964 :`B` 1.0 :`A` 1.0) (`self.RL`))
          (if (`self.DrawDebug`)
            (`KismetSystemLibrary.DrawDebugPoint` (0.0 0.0 0.0) 30.0 (struct :`G` 0.411144 :`B` 1.0 :`A` 1.0))))))
    (:`then_1`
      (if (`self.AllowOptimization`)
        (if (< _returnvalue_2 1000.0)
          (`self.SetActorTickInterval` 0.15)
          (elif (>= _returnvalue_2 1000.0)
            (`self.SetActorTickInterval` 0.2)
            (elif (>= _returnvalue_2 2000.0)
              (`self.SetActorTickInterval` 0.5)
              (elif (>= _returnvalue_2 4000.0)
                (`self.SetActorTickInterval` 1.0)))))))))

(event `self.ReceiveBeginPlay`
  (bind _fl (`self.FL`))
  (bind _rl (`self.RL`))
  (bind _rr (`self.RR`))
  (bind _fr (`self.FR`))
  (bind _asbp_third_person_character (cast `/Game/Rome/Demo/PawnUE5/Demo/EpicContent/ThirdPersonBP/Blueprints/BP_ThirdPersonCharacter` (`GameplayStatics.GetPlayerCharacter` 0)))
  (set `self.Character Reference` _asbp_third_person_character)
  (`|ExecutionSequence`
    (:`then_0`
      (`AudioComponent.SetSound` _fl (`self.Front Left`))
      (`AudioComponent.Play` _fl 0.0))
    (:`then_1`
      (`AudioComponent.SetSound` _fr (`self.Front Right`))
      (`AudioComponent.Play` _fr 0.0))
    (:`then_2`
      (`AudioComponent.SetSound` _rl (`self.Rear Left`))
      (`AudioComponent.Play` _rl 0.0))
    (:`then_3`
      (`AudioComponent.SetSound` _rr (`self.Rear Right`))
      (`AudioComponent.Play` _rr 0.0))))

(event `ConstrainPoint`
  (params (Point :type "Vector Structure") (PointColor :type "LinearColor Structure") (`Audio Emitter` :type "AudioComponent Object Reference"))
  (bind _box (`self.Box`))
  (bind _pointonsurface (`self.ClampPointOnSurface` Point (`BoxComponent.GetScaledBoxExtent` _box) (`SceneComponent.K2_GetComponentToWorld` _box)))
  (`SceneComponent.K2_SetWorldLocation` `Audio Emitter` _pointonsurface false false)
  (if (`self.DrawDebug`)
    (`KismetSystemLibrary.DrawDebugSphere` _pointonsurface 4.0 12 PointColor 0.0 1.0)))

(fn `CalculateEmitterPositions`
  (params (PawnLocation :type "Vector Structure") (PawnRotation :type "Rotator Structure") (PointsDistanceFromCenter :type "Float (double-precision)"))
  (returns (Front :type "Vector Structure") (Right :type "Vector Structure") (Back :type "Vector Structure") (Left :type "Vector Structure"))
  (bind _returnvalue (* (`KismetMathLibrary.GetRightVector` PawnRotation) PointsDistanceFromCenter))
  (bind _returnvalue_2 (* (`KismetMathLibrary.GetForwardVector` PawnRotation) PointsDistanceFromCenter))
  (return (+ PawnLocation _returnvalue_2) (+ PawnLocation _returnvalue) (+ PawnLocation (* _returnvalue_2 -1.0)) (+ PawnLocation (* _returnvalue -1.0))))

(fn `ClampLocalPoint`
  (params (Point :type "Vector Structure") (Extent :type "Vector Structure"))
  (returns (ClampedPoint :type "Vector Structure"))
  (locals (ClampedLocalPoint :type "Vector Structure"))
  (bind _x (.x Extent))
  (bind _y (.y Extent))
  (bind _z (.z Extent))
  (return (`KismetMathLibrary.MakeVector` (`KismetMathLibrary.FClamp` (.x Point) (* _x -1.0) _x) (`KismetMathLibrary.FClamp` (.y Point) (* _y -1.0) _y) (`KismetMathLibrary.FClamp` (.z Point) (* _z -1.0) _z))))

(fn `ClampPointOnSurface`
  (params (Point :type "Vector Structure") (Extent :type "Vector Structure") (CuboidTransform :type "Transform Structure"))
  (returns (PointOnSurface :type "Vector Structure"))
  (locals (LocalPoint :type "Vector Structure") (WorldClampedPoint :type "Vector Structure") (ClampedLocalPoint :type "Vector Structure"))
  (`|ExecutionSequence`
    (:`then_1`
      ;[1 1 1] Convert Point to Cuboid Space
      (set `local.LocalPoint` (`KismetMathLibrary.InverseTransformLocation` CuboidTransform Point)))
    (:`then_2`
      ;[1 1 1] Clamp Point
      (set `local.ClampedLocalPoint` (`self.ClampLocalPoint` (`local.LocalPoint`) Extent)))
    (:`then_3`
      ;[1 1 1] Convert Point back to World Space
      (set `local.WorldClampedPoint` (`KismetMathLibrary.TransformLocation` CuboidTransform (`local.ClampedLocalPoint`))))
    (:`then_4`
      ;[1 1 1] Return calculated Value
      (return (`local.WorldClampedPoint`)))))

(fn `UserConstructionScript`)