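; Actor that surrounds the player with a four-channel sound bed from front-left, front-right, rear-left and rear-right audio components.
; On BeginPlay it assigns and plays a sound on each emitter and caches the player's BP_ThirdPersonCharacter.
; Every tick it moves its root to the character's head socket.
; It subtracts the camera rotation from itself, keeping world rotation at zero, so emitters ignore where the player looks.
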(event `self.ReceiveBeginPlay`
  (bind _fl (`self.FL`))
  (bind _rl (`self.RL`))
  (bind _rr (`self.RR`))
  (bind _fr (`self.FR`))
  (`|ExecutionSequence`
    (:`then_0`
      (`AudioComponent.SetSound` _fl (`self.Front Left`))
      (`AudioComponent.Play` _fl 0.0)
      (bind _asbp_third_person_character (cast `/Game/Rome/Demo/PawnUE5/Demo/EpicContent/ThirdPersonBP/Blueprints/BP_ThirdPersonCharacter` (`GameplayStatics.GetPlayerCharacter` 0)))
      (set `self.Character Reference` _asbp_third_person_character))
    (:`then_1`
      (`AudioComponent.SetSound` _fr (`self.Front Right`))
      (`AudioComponent.Play` _fr 0.0))
    (:`then_2`
      (`AudioComponent.SetSound` _rl (`self.Rear Left`))
      (`AudioComponent.Play` _rl 0.0))
    (:`then_3`
      (`AudioComponent.SetSound` _rr (`self.Rear Right`))
      (`AudioComponent.Play` _rr 0.0))))

(event `self.ReceiveTick`
  (params (DeltaSeconds :type "Float (single-precision)"))
  (bind _character_reference (`self.Character Reference`))
  (bind _defaultsceneroot (`self.DefaultSceneRoot`))
  (bind _fppcamera (`/Game/Rome/Demo/PawnUE5/Demo/EpicContent/ThirdPersonBP/Blueprints/BP_ThirdPersonCharacter.FPPCamera` _character_reference))
  (bind (_returnvalue_roll _returnvalue_pitch _returnvalue_yaw) (`KismetMathLibrary.BreakRotator` (`SceneComponent.K2_GetComponentRotation` _fppcamera)))
  (bind (_returnvalue_roll_2 _returnvalue_pitch_2 _returnvalue_yaw_2) (`KismetMathLibrary.BreakRotator` (`SceneComponent.K2_GetComponentRotation` _fppcamera)))
  (`SceneComponent.K2_SetWorldRotation` _defaultsceneroot (`KismetMathLibrary.MakeRotator` (- _returnvalue_roll _returnvalue_roll_2) (- _returnvalue_pitch _returnvalue_pitch_2) (- _returnvalue_yaw _returnvalue_yaw_2)) false false)
  (`SceneComponent.K2_SetWorldLocation` _defaultsceneroot (`SceneComponent.GetSocketLocation` (`Character.Mesh` _character_reference) "head") false false))

(fn `UserConstructionScript`)